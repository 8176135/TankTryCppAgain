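; TankState holds per-tank respawn and boost state, though most of its logic is currently disconnected.
; BeginPlay creates and stores a RespawnHud widget, and ResetRestables clears the Boosted flag.
; The other events are empty stubs, leaving the respawn timer, HUD progress bar and alive-state logic in unreachable chains.
; The BoostFuel RepNotify is also empty, with its player fuel update left unwired.
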(event Custom|StartRespawnTimer)

(event Custom|MakeRespawnHud)

(event Custom|RemoveAndResetRsScreen)

(event Custom|AllowRespawn)

(event Custom|Respawned)

(event Custom|ResetRestables
  (Variables|Default|SetBoosted false))

(event EventTick
  (params (DeltaSeconds :type Float%20%28single-precision%29)))

(event EventBeginPlay
  (bind _returnvalue (UserInterface|CreateWidget "/Game/UI/RespawnHud.RespawnHud_C"))
  (Variables|Default|SetResHud _returnvalue))

(fn ConstructionScript)

(fn OnRepBoostFuel)