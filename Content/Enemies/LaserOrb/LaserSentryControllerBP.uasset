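; AI controller for the laser orb sentry, running its behavior tree and steering it through blackboard state.
; On possess it waits for the player's TankState, then starts a looping Check timer that is cleared on unpossess.
; Unless State is 2, Check finds the nearest target if none is valid, or range-checks and line-traces to it.
; Hitting a Turret-tagged actor sets State 1 and pulses AbortAndReset; otherwise State returns to 0.
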(event Custom|Check
  (bind _returnvalue (Pawn|GetControlledPawn))
  (bind _returnvalue_2 (Utilities|Name|MakeLiteralName "State"))
  (bind _returnvalue_3 (Utilities|Name|MakeLiteralName "AbortAndReset"))
  (bind _blackboard (Variables|Default|GetBlackboard))
  (bind _returnvalue_4 (Transformation|GetActorLocation _returnvalue))
  (if (!= (Class|BlackboardComponent|GetValueasEnum (Variables|Default|GetBlackboard) (Utilities|Name|MakeLiteralName "State")) 2)
    (Utilities|IsValid (Variables|Default|GetAiTarget)
      (:Is%20Valid
        (if (< (Math|Vector|VectorLength (- (Transformation|GetActorLocation (Variables|Default|GetAiTarget)) _returnvalue_4)) (Variables|Default|GetDistance))
          (bind (_outhit _returnvalue_5) (Collision|LineTraceForObjects _returnvalue_4 (+ (Transformation|GetActorLocation (Variables|Default|GetAiTarget)) "0.000000, 0,5.000000") (Variables|Default|GetpathBlockingObjects) false (Utilities|Array|MakeArray (Pawn|GetControlledPawn)) "None" true "(R=1.000000,G=0.000000,B=0.000000,A=1.000000)" "(R=0.000000,G=1.000000,B=0.000000,A=1.000000)" 1.0))
          (if _returnvalue_5
            (if (Actor|ActorHasTag (.HitActor (Collision|BreakHitResult _outhit)) "Turret")
              (if (== (.HitActor (Collision|BreakHitResult _outhit)) (Variables|Default|GetAiTarget))
                _
                (else
                  (Development|PrintString "Well the impossible just happened")
                  (Variables|Default|SetAiTarget (.HitActor (Collision|BreakHitResult _outhit)))))
              (AI|Components|Blackboard|SetValueasEnum _blackboard _returnvalue_2 1)
              (AI|Components|Blackboard|SetValueasBool _blackboard _returnvalue_3 false)
              (AI|Components|Blackboard|SetValueasBool _blackboard _returnvalue_3 true)
              (else
                (AI|Components|Blackboard|SetValueasEnum (Variables|Default|GetBlackboard) _returnvalue_2 :!label _label)))
            (else
              (Development|PrintString "Wtf, something is wrong with the turret collision]")
              (goto _label)))
          (else
            (AI|Components|Blackboard|SetValueasEnum (Variables|Default|GetBlackboard) _returnvalue_2))))
      (:Is%20Not%20Valid
        (Utilities|FlowControl|Delay 0.1)
        (Class|LaserSentryController|FindNearestTarget (delegate Custom|Data%20Return))))))

(event Custom|Data%20Return
  (params (newTargetActor :type Base%20Turret%20Object%20Reference) (successful :type Boolean))
  (if successful
    (bind _output_get (Variables|Default|SetAiTarget newTargetActor))
    (AI|Components|Blackboard|SetValueasObject (Variables|Default|GetBlackboard) (Utilities|Name|MakeLiteralName "TargetAct") _output_get)
    (else
      (Development|PrintString "Failed to find a target"))))

(event EventBeginPlay)

(event EventOnPossess
  (params (PossessedPawn :type Pawn%20Object%20Reference))
  (bind _returnvalue (Game|GetPlayerController 0))
  (Utilities|IsValid _returnvalue
    (:Is%20Valid
      (Utilities|Casting|CastToTankState (Variables|/Script/Engine.Controller|GetPlayerState _returnvalue) :!label _label
        (:then
          _)
        (:CastFailed
          (Utilities|FlowControl|Delay 0.2 :!label _label_2)
          (goto _label))))
    (:Is%20Not%20Valid
      (goto _label_2)))
  (AI|RunBehaviorTree "/Game/Enemies/LaserOrb/LaserOrbBehaviour.LaserOrbBehaviour")
  (bind _returnvalue_2 (Utilities|Time|SetTimerbyEvent (delegate Custom|Check) 0.5 true))
  (Variables|Default|SetCheckTimer _returnvalue_2))

(event EventOnUnpossess
  (params (UnpossessedPawn :type Pawn%20Object%20Reference))
  (Utilities|Time|ClearandInvalidateTimerbyHandle (Variables|Default|GetCheckTimer)))

(fn ConstructionScript)