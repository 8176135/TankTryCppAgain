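; Player controller for the aerial tank that handles the player's respawn request.
; BeginPlay caches the TankState player state; the Respawn input triggers RequestRespawn only when no valid pawn is controlled, otherwise printing a debug message.
; After a short delay, RequestRespawn checks TankState.AbleToRespawn, printing a wait message if false.
; If allowed, only the authority branch resets the respawn screen through TankState and passes the controller to FirstPersonGameMode's RespawningSt.
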(event Custom|RequestRespawn
  (bind _returnvalue (Game|GetGameMode))
  (Utilities|FlowControl|Delay 0.1)
  (if (Variables|/Game/Blueprints/TankState.TankState_C|GetAbleToRespawn (Variables|Default|GetTankState))
    (Networking|SwitchHasAuthority
      (:Authority
        (Utilities|IsValid _returnvalue
          (:Is%20Valid
            (bind _asfirst_person_game_mode (Utilities|Casting|CastToFirstPersonGameMode _returnvalue))
            (Utilities|IsValid _asfirst_person_game_mode
              (:Is%20Valid
                (Default|RemoveandResetRsScreen (Variables|Default|GetTankState))
                (Default|RespawningSt _asfirst_person_game_mode self)))))))
    (else
      (Development|PrintString "Wait..."))))

(event EventBeginPlay
  (bind _astank_state (Utilities|Casting|CastToTankState (Variables|GetPlayerState)))
  (Variables|Default|SetTankState _astank_state))

(event EventTick
  (params (DeltaSeconds :type Float%20%28single-precision%29)))

(event Input|ActionEvents|InputActionRespawn
  (params (Key :type Key%20Structure :default "AnyKey"))
  (:Pressed
    (Utilities|IsValid (Pawn|GetControlledPawn)
      (:Is%20Valid
        (Development|PrintString "UR STILL ALVIE!"))
      (:Is%20Not%20Valid
        (CallFunction|RequestRespawn)))))

(fn ConstructionScript)